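; BP_Lord is a tower-defense lord actor with health and a summon ability, reporting to BP_TDGameDirector.
; TakeTDamage subtracts HP and at zero notifies the director of the lord's death, then destroys the actor.
; CastAbility, gated by a game-time cooldown, has the director spawn free ghouls on the four orthogonally adjacent grid tiles.
; Both functions find the director by class lookup, and the event graph is empty.
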(fn `CastAbility`
  (bind _returnvalue (`KismetSystemLibrary.GetGameTimeInSeconds`))
  (if (>= _returnvalue (`self.AbilityCd`))
    (set `self.AbilityCd` (+ _returnvalue 60.0))
    (bind _outactors (`GameplayStatics.GetAllActorsOfClass` "/Game/Blueprints/BP_TDGameDirector.BP_TDGameDirector_C"))
    (if (> (`KismetArrayLibrary.Array_Length` _outactors) 0)
      (bind _asbp_tdgame_director (cast `/Game/Blueprints/BP_TDGameDirector` (`|GetArrayItem` _outactors))
        (:`then`
          (bind (_col _row) (`/Game/Blueprints/BP_TDGameDirector.WorldToTile` _asbp_tdgame_director (`self.K2_GetActorLocation`)))
          (`/Game/Blueprints/BP_TDGameDirector.SpawnFreeUnit` _asbp_tdgame_director "ghoul" (+ _col 1) _row)
          (`/Game/Blueprints/BP_TDGameDirector.SpawnFreeUnit` _asbp_tdgame_director "ghoul" (- _col 1) _row)
          (`/Game/Blueprints/BP_TDGameDirector.SpawnFreeUnit` _asbp_tdgame_director "ghoul" _col (+ _row 1))
          (`/Game/Blueprints/BP_TDGameDirector.SpawnFreeUnit` _asbp_tdgame_director "ghoul" _col (- _row 1)))
        (:`CastFailed`
          (`KismetSystemLibrary.PrintString` "CastAbility: director cast failed")))
      (else
        (`KismetSystemLibrary.PrintString` "CastAbility: no director")))))

(fn `TakeTDamage`
  (params (N :type "Float (double-precision)"))
  (set `self.HP` (- (`self.HP`) N))
  (if (<= (`self.HP`) 0.0)
    (bind _outactors (`GameplayStatics.GetAllActorsOfClass` "/Game/Blueprints/BP_TDGameDirector.BP_TDGameDirector_C"))
    (if (> (`KismetArrayLibrary.Array_Length` _outactors) 0)
      (bind _asbp_tdgame_director (cast `/Game/Blueprints/BP_TDGameDirector` (`|GetArrayItem` _outactors))
        (:`then`
          (`/Game/Blueprints/BP_TDGameDirector.NotifyLordDead` _asbp_tdgame_director)
          (`self.K2_DestroyActor` self))
        (:`CastFailed`
          (`self.K2_DestroyActor` self)))
      (else
        (`self.K2_DestroyActor` self)))))

(fn `UserConstructionScript`)