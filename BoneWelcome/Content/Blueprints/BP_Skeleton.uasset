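; Skeleton minion that guards a home point, chasing and striking nearby BP_Unit actors, and reports its death to its owning BP_Tower.
; A looping 0.1-second timer replaces Tick, picking the unit nearest home within leash range, then attacking on cooldown or stepping toward it by unswept teleport.
; Without a target it walks back home.
; Init sets home, health and a scaled cylinder placeholder look, while InitSkel only sets home.
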(event `self.ReceiveBeginPlay`
  (`KismetSystemLibrary.K2_SetTimer` self "TickMove" 0.1 true))

(fn `FindNearestUnitHome`
  (params (MaxDist :type "Float (double-precision)"))
  (returns (OutActor :type "Actor Object Reference"))
  (bind _outactors (`GameplayStatics.GetAllActorsOfClass` "/Game/Blueprints/BP_Unit.BP_Unit_C"))
  (set `self.SBestIdx` -1)
  (set `self.SBestDist` MaxDist)
  (for _index (range (+ (- (`KismetArrayLibrary.Array_Length` _outactors) 1) 1))
    (bind _returnvalue (`KismetMathLibrary.Vector_Distance2D` (`self.Home`) (`self.K2_GetActorLocation` (`|GetArrayItem` _outactors _index))))
    (if (< _returnvalue (`self.SBestDist`))
      (set `self.SBestDist` _returnvalue)
      (set `self.SBestIdx` _index)))
  (if (>= (`self.SBestIdx`) 0)
    (return (`|GetArrayItem` _outactors (`self.SBestIdx`)))
    (else
      (return null))))

(fn `Init`
  (params (HomeV :type "Vector Structure"))
  (set `self.Home` HomeV)
  (set `self.HP` 60.0)
  (bind _asstatic_mesh_component (cast `StaticMeshComponent` (`self.GetComponentByClass` self "/Script/Engine.StaticMeshComponent")))
  (`StaticMeshComponent.SetStaticMesh` _asstatic_mesh_component "/Engine/BasicShapes/Cylinder.Cylinder")
  (`PrimitiveComponent.SetMaterial` _asstatic_mesh_component 0 "/Game/Materials/M_BoneWall.M_BoneWall")
  (`self.SetActorScale3D` self (`KismetMathLibrary.MakeVector` 0.45 0.45 0.9)))

(fn `InitSkel`
  (params (Home :type "Vector Structure"))
  (set `self.Home` Home)
  (set `self.HomeLocation` Home))

(fn `TakeTDamage`
  (params (N :type "Float (double-precision)"))
  (if (not (`self.bDead`))
    (set `self.HP` (- (`self.HP`) N))
    (if (<= (`self.HP`) 0.0)
      (set `self.bDead` true)
      (`/Engine/EditorBlueprintResources/StandardMacros.IsValid` (`self.HomeTower`)
        (:`Is Valid`
          (bind _asbp_tower (cast `/Game/Blueprints/BP_Tower` (`self.HomeTower`))
            (:`then`
              (`/Game/Blueprints/BP_Tower.ChildDied` _asbp_tower self)
              (`self.K2_DestroyActor` self))
            (:`CastFailed`
              (`self.K2_DestroyActor` self))))
        (:`Is Not Valid`
          (`self.K2_DestroyActor` self))))))

(fn `TickMove`
  (bind _returnvalue (`self.K2_GetActorLocation`))
  (bind _returnvalue_2 (`self.K2_GetActorLocation`))
  (bind _home (`self.Home`))
  (bind _returnvalue_3 (`KismetMathLibrary.Vector_Distance2D` _returnvalue_2 _home))
  (if (not (`self.bDead`))
    (set `self.AtkCD` (- (`self.AtkCD`) 0.1))
    (bind _outactor (`self.FindNearestUnitHome` 500.0))
    (`/Engine/EditorBlueprintResources/StandardMacros.IsValid` _outactor
      (:`Is Valid`
        (bind _returnvalue_4 (`self.K2_GetActorLocation` _outactor))
        (bind _returnvalue_5 (`KismetMathLibrary.Vector_Distance2D` _returnvalue _returnvalue_4))
        (if (<= _returnvalue_5 130.0)
          (if (<= (`self.AtkCD`) 0.0)
            (set `self.AtkCD` 1.0)
            (bind _asbp_unit (cast `/Game/Blueprints/BP_Unit` _outactor))
            (`/Game/Blueprints/BP_Unit.TakeTDamage` _asbp_unit 8.0))
          (elif (> _returnvalue_5 1.0)
            (`self.K2_SetActorLocation` self (`KismetMathLibrary.MakeVector` (+ (.x _returnvalue) (* 260.0 (* 0.1 (/ (- (.x _returnvalue_4) (.x _returnvalue)) _returnvalue_5)))) (+ (.y _returnvalue) (* 260.0 (* 0.1 (/ (- (.y _returnvalue_4) (.y _returnvalue)) _returnvalue_5)))) (.z _returnvalue)) false true))))
      (:`Is Not Valid`
        (if (> _returnvalue_3 90.0)
          (`self.K2_SetActorLocation` self (`KismetMathLibrary.MakeVector` (+ (.x _returnvalue_2) (* 260.0 (* 0.1 (/ (- (.x _home) (.x _returnvalue_2)) _returnvalue_3)))) (+ (.y _returnvalue_2) (* 260.0 (* 0.1 (/ (- (.y _home) (.y _returnvalue_2)) _returnvalue_3)))) (.z _returnvalue_2)) false true))))))

(fn `UserConstructionScript`)