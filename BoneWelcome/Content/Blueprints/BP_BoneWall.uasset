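; Destructible bone wall for a tile-based tower defense, whose death releases a burst of skeletons.
; TakeTDamage drains HP; at zero it scans the BP_TDGameDirector tile grid for the nearest "T" tile.
; It spawns a row of skeletons there through the director, reports the wall down, awards souls and destroys itself.
; TakeDmg is an empty stub, and disconnected older copies of the damage logic remain.
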(fn `TakeDmg`
  (params (Amount :type "Float (double-precision)")))

(fn `TakeTDamage`
  (params (N :type "Float (double-precision)"))
  (set `self.HP` (- (`self.HP`) N))
  (if (<= (`self.HP`) 0.0)
    (bind _outactors (`GameplayStatics.GetAllActorsOfClass` "/Game/Blueprints/BP_TDGameDirector.BP_TDGameDirector_C"))
    (if (> (`KismetArrayLibrary.Array_Length` _outactors) 0)
      (bind _asbp_tdgame_director (cast `/Game/Blueprints/BP_TDGameDirector` (`|GetArrayItem` _outactors))
        (:`then`
          (set `self.WBestDist` 99999999.0)
          (for _index (range 64)
            (for _index_2 (range 24)
              (bind _char (`/Game/Blueprints/BP_TDGameDirector.TileChar` _asbp_tdgame_director _index _index_2))
              (if (`KismetStringLibrary.EqualEqual_StrStr` _char "T")
                (bind _pos (`/Game/Blueprints/BP_TDGameDirector.TileToWorld` _asbp_tdgame_director _index _index_2))
                (if (< (`KismetMathLibrary.Vector_Distance2D` (`self.K2_GetActorLocation`) _pos) (`self.WBestDist`))
                  (bind _pos_2 (`/Game/Blueprints/BP_TDGameDirector.TileToWorld` _asbp_tdgame_director _index _index_2))
                  (set `self.WBestDist` (`KismetMathLibrary.Vector_Distance2D` (`self.K2_GetActorLocation`) _pos_2))
                  (bind _pos_3 (`/Game/Blueprints/BP_TDGameDirector.TileToWorld` _asbp_tdgame_director _index _index_2))
                  (set `self.WBestPos` _pos_3)))))
          (if (< (`self.WBestDist`) 9999999.0)
            (for _index_3 (range 6)
              (`/Game/Blueprints/BP_TDGameDirector.SpawnSkeletonAt` _asbp_tdgame_director (`KismetMathLibrary.MakeVector` (+ (.x (`self.WBestPos`)) (- (* 60.0 _index_3) 150.0)) (.y (`self.WBestPos`)) 20.0))))
          (`/Game/Blueprints/BP_TDGameDirector.NotifyWallDown` _asbp_tdgame_director)
          (`/Game/Blueprints/BP_TDGameDirector.AddSoul` _asbp_tdgame_director 20)
          (`self.K2_DestroyActor` self))
        (:`CastFailed`
          (`self.K2_DestroyActor` self)))
      (else
        (`self.K2_DestroyActor` self)))))

(fn `UserConstructionScript`)