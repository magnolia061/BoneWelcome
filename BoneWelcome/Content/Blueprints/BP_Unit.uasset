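; BP_Unit is a tower-defense combat unit configured as ghoul, archer, troll or apostle, each with its own stats and tinted cylinder.
; A looping 0.1-second timer replaces Tick, running attack cooldown, poison, slow and fear, which makes it flee its source.
; Otherwise it follows grid paths from BP_TDGameDirector, then closes on any commanded target and attacks within range.
; Damage dispatches by class cast; death notifies the director and destroys the actor.
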(event `self.ReceiveBeginPlay`
  (`self.InitUnit` (`self.UnitType`))
  (`KismetSystemLibrary.K2_SetTimer` self "TickMove" 0.1 true))

(fn `ApplyFear`
  (params (Dur :type "Float (double-precision)") (SrcX :type "Float (double-precision)") (SrcY :type "Float (double-precision)"))
  (if (!= 0 2)
    (set `self.FearT` Dur)
    (set `self.FearSrcX` SrcX)
    (set `self.FearSrcY` SrcY)))

(fn `ApplyPoison`
  (params (DPS :type "Float (double-precision)") (Dur :type "Float (double-precision)"))
  (if (!= 0 3)
    (set `self.PoisonDPS` DPS)
    (set `self.PoisonT` Dur)
    (set `self.SlowT` Dur)))

(fn `DealDamageTo`
  (params (T :type "Actor Object Reference"))
  (bind _asbp_tower (cast `/Game/Blueprints/BP_Tower` T)
    (:`then`
      (`/Game/Blueprints/BP_Tower.TakeTDamage` _asbp_tower (`self.Atk`)))
    (:`CastFailed`
      (bind _asbp_gate (cast `/Game/Blueprints/BP_Gate` T)
        (:`then`
          (`/Game/Blueprints/BP_Gate.TakeTDamage` _asbp_gate (`self.Atk`)))
        (:`CastFailed`
          (bind _asbp_bone_wall (cast `/Game/Blueprints/BP_BoneWall` T)
            (:`then`
              (`/Game/Blueprints/BP_BoneWall.TakeTDamage` _asbp_bone_wall (`self.Atk`)))
            (:`CastFailed`
              (bind _asbp_skeleton (cast `/Game/Blueprints/BP_Skeleton` T)
                (:`then`
                  (`/Game/Blueprints/BP_Skeleton.TakeTDamage` _asbp_skeleton (`self.Atk`)))
                (:`CastFailed`
                  (bind _asbp_unit (cast `/Game/Blueprints/BP_Unit` T))
                  (`self.TakeTDamage` _asbp_unit (`self.Atk`)))))))))))

(fn `EngageTarget`
  (params (T :type "Actor Object Reference") (Spd :type "Float (double-precision)"))
  (bind _returnvalue (`self.K2_GetActorLocation`))
  (bind _returnvalue_2 (`self.K2_GetActorLocation` T))
  (bind _returnvalue_3 (`KismetMathLibrary.Vector_Distance2D` _returnvalue _returnvalue_2))
  (if (<= _returnvalue_3 (`self.Range`))
    (if (<= (`self.AtkCD`) 0.0)
      (set `self.AtkCD` (`self.AtkInterval`))
      (`self.DealDamageTo` T))
    (elif (> _returnvalue_3 1.0)
      (`self.K2_SetActorLocation` self (`KismetMathLibrary.MakeVector` (+ (.x _returnvalue) (* Spd (* 0.1 (/ (- (.x _returnvalue_2) (.x _returnvalue)) _returnvalue_3)))) (+ (.y _returnvalue) (* Spd (* 0.1 (/ (- (.y _returnvalue_2) (.y _returnvalue)) _returnvalue_3)))) (.z _returnvalue)) false true))))

(fn `FindNearestOf`
  (params (Arr :type "Array of Actor Object Reference") (Loc :type "Vector Structure") (MaxDist :type "Float (double-precision)"))
  (returns (OutActor :type "Actor Object Reference"))
  (set `self.PBestIdx` -1)
  (set `self.PBestDist` MaxDist)
  (for _index (range (+ (- (`KismetArrayLibrary.Array_Length` Arr) 1) 1))
    (bind _returnvalue (`KismetMathLibrary.Vector_Distance2D` Loc (`self.K2_GetActorLocation` (`|GetArrayItem` Arr _index))))
    (if (< _returnvalue (`self.PBestDist`))
      (set `self.PBestDist` _returnvalue)
      (set `self.PBestIdx` _index)))
  (if (>= (`self.PBestIdx`) 0)
    (return (`|GetArrayItem` Arr (`self.PBestIdx`)))
    (else
      (return null))))

(fn `FollowPath`
  (params (Spd :type "Float (double-precision)"))
  (bind _returnvalue (`self.K2_GetActorLocation`))
  (bind _output (`|GetArrayItem` (`self.Path`) (`self.PathIdx`)))
  (bind _returnvalue_2 (`KismetMathLibrary.Vector_Distance2D` _returnvalue _output))
  (if (< (`self.PathIdx`) (`KismetArrayLibrary.Array_Length` (`self.Path`)))
    (if (< _returnvalue_2 60.0)
      (set `self.PathIdx` (+ (`self.PathIdx`) 1))
      (else
        (`self.K2_SetActorLocation` self (`KismetMathLibrary.MakeVector` (+ (.x _returnvalue) (* Spd (* 0.1 (/ (- (.x _output) (.x _returnvalue)) _returnvalue_2)))) (+ (.y _returnvalue) (* Spd (* 0.1 (/ (- (.y _output) (.y _returnvalue)) _returnvalue_2)))) (.z _returnvalue)) false true)))))

(fn `Init`
  (params (TypeIdx :type Integer) (D :type "Actor Object Reference"))
  (set `self.Director` D)
  (if (== TypeIdx 1)
    (set `self.UnitType` "archer")
    (set `self.MaxHP` 80.0)
    (set `self.HP` 80.0)
    (set `self.Atk` 15.0)
    (set `self.Range` 500.0)
    (set `self.AtkInterval` 1.0)
    (set `self.MoveSpeed` 210.0)
    (set `self.Speed` 210.0)
    (`self.SetupVisual`)
    (elif (== TypeIdx 2)
      (set `self.UnitType` "troll")
      (set `self.MaxHP` 800.0)
      (set `self.HP` 800.0)
      (set `self.Atk` 30.0)
      (set `self.Range` 140.0)
      (set `self.AtkInterval` 1.2)
      (set `self.MoveSpeed` 150.0)
      (set `self.Speed` 150.0)
      (`self.SetupVisual`)
      (elif (== TypeIdx 3)
        (set `self.UnitType` "apostle")
        (set `self.MaxHP` 200.0)
        (set `self.HP` 200.0)
        (set `self.Atk` 20.0)
        (set `self.Range` 300.0)
        (set `self.AtkInterval` 1.0)
        (set `self.MoveSpeed` 190.0)
        (set `self.Speed` 190.0)
        (`self.SetupVisual`)
        (else
          (set `self.UnitType` "ghoul")
          (set `self.MaxHP` 120.0)
          (set `self.HP` 120.0)
          (set `self.Atk` 10.0)
          (set `self.Range` 140.0)
          (set `self.AtkInterval` 1.0)
          (set `self.MoveSpeed` 240.0)
          (set `self.Speed` 240.0)
          (`self.SetupVisual`))))))

(fn `InitUnit`
  (params (UnitType :type Name))
  (if (== UnitType "archer")
    (set `self.UnitType` "archer")
    (set `self.MaxHP` 80.0)
    (set `self.HP` 80.0)
    (set `self.Atk` 15.0)
    (set `self.Range` 500.0)
    (set `self.AtkInterval` 1.0)
    (set `self.MoveSpeed` 210.0)
    (set `self.Speed` 210.0)
    (`self.SetupVisual`)
    (elif (== UnitType "troll")
      (set `self.UnitType` "troll")
      (set `self.MaxHP` 800.0)
      (set `self.HP` 800.0)
      (set `self.Atk` 30.0)
      (set `self.Range` 140.0)
      (set `self.AtkInterval` 1.2)
      (set `self.MoveSpeed` 150.0)
      (set `self.Speed` 150.0)
      (`self.SetupVisual`)
      (elif (== UnitType "apostle")
        (set `self.UnitType` "apostle")
        (set `self.MaxHP` 200.0)
        (set `self.HP` 200.0)
        (set `self.Atk` 20.0)
        (set `self.Range` 300.0)
        (set `self.AtkInterval` 1.0)
        (set `self.MoveSpeed` 190.0)
        (set `self.Speed` 190.0)
        (`self.SetupVisual`)
        (else
          (set `self.UnitType` "ghoul")
          (set `self.MaxHP` 120.0)
          (set `self.HP` 120.0)
          (set `self.Atk` 10.0)
          (set `self.Range` 140.0)
          (set `self.AtkInterval` 1.0)
          (set `self.MoveSpeed` 240.0)
          (set `self.Speed` 240.0)
          (`self.SetupVisual`))))))

(fn `RepathTo`
  (params (Loc :type "Vector Structure"))
  (bind _returnvalue (`self.K2_GetActorLocation`))
  (bind _asbp_tdgame_director (cast `/Game/Blueprints/BP_TDGameDirector` (`self.Director`)))
  (bind _path (`/Game/Blueprints/BP_TDGameDirector.FindPath` _asbp_tdgame_director (`KismetMathLibrary.FFloor` (/ (.x _returnvalue) 100.0)) (`KismetMathLibrary.FFloor` (/ (.y _returnvalue) 100.0)) (`KismetMathLibrary.FFloor` (/ (.x Loc) 100.0)) (`KismetMathLibrary.FFloor` (/ (.y Loc) 100.0))))
  (set `self.Path` _path)
  (set `self.PathIdx` 0))

(fn `SetMoveCommand`
  (params (Loc :type "Vector Structure"))
  (set `self.MoveTarget` Loc)
  (set `self.bHasMoveCmd` true)
  (set `self.bHasTargetCmd` false)
  (`self.RepathTo` Loc))

(fn `SetTargetCommand`
  (params (T :type "Actor Object Reference"))
  (set `self.TargetActor` T)
  (set `self.bHasTargetCmd` true)
  (set `self.bHasMoveCmd` false))

(fn `SetupVisual`
  (bind _asstatic_mesh_component (cast `StaticMeshComponent` (`self.GetComponentByClass` self "/Script/Engine.StaticMeshComponent")))
  (`StaticMeshComponent.SetStaticMesh` _asstatic_mesh_component "/Engine/BasicShapes/Cylinder.Cylinder")
  (if (== (`self.UnitType`) "ghoul")
    (`PrimitiveComponent.SetMaterial` _asstatic_mesh_component 0 "/Game/Materials/M_Player.M_Player")
    (`self.SetActorScale3D` self (`KismetMathLibrary.MakeVector` 0.6 0.6 1.3))
    (elif (== (`self.UnitType`) "archer")
      (`PrimitiveComponent.SetMaterial` _asstatic_mesh_component 0 "/Game/Materials/M_SoulGlow.M_SoulGlow")
      (`self.SetActorScale3D` self (`KismetMathLibrary.MakeVector` 0.5 0.5 1.1))
      (elif (== (`self.UnitType`) "troll")
        (`PrimitiveComponent.SetMaterial` _asstatic_mesh_component 0 "/Game/Materials/M_BoneWall.M_BoneWall")
        (`self.SetActorScale3D` self (`KismetMathLibrary.MakeVector` 1.3 1.3 2.2))
        (else
          (`PrimitiveComponent.SetMaterial` _asstatic_mesh_component 0 "/Game/Materials/M_PoisonGlow.M_PoisonGlow")
          (`self.SetActorScale3D` self (`KismetMathLibrary.MakeVector` 0.7 0.7 1.5)))))))

(fn `TakeTDamage`
  (params (N :type "Float (double-precision)"))
  (if (not (`self.bDead`))
    (set `self.HP` (- (`self.HP`) N))
    (if (<= (`self.HP`) 0.0)
      (set `self.bDead` true)
      (bind _asbp_tdgame_director (cast `/Game/Blueprints/BP_TDGameDirector` (`self.Director`))
        (:`then`
          (`/Game/Blueprints/BP_TDGameDirector.NotifyUnitDead` _asbp_tdgame_director self)
          (`self.K2_DestroyActor` self))
        (:`CastFailed`
          (`self.K2_DestroyActor` self))))))

(fn `TickMove`
  (bind _returnvalue (`self.K2_GetActorLocation`))
  (bind _returnvalue_2 (`KismetMathLibrary.Vector_Distance2D` _returnvalue (`KismetMathLibrary.MakeVector` (`self.FearSrcX`) (`self.FearSrcY`) (.z _returnvalue))))
  (bind _returnvalue_3 (* (`self.MoveSpeed`) (select `bool` (> (`self.SlowT`) 0.0) :`false` 1.0 :`true` 0.6)))
  (if (not (<= (`self.HP`) 0.0))
    (set `self.AtkCD` (- (`self.AtkCD`) 0.1))
    (`self.TakeTDamage` (* (`self.PoisonDPS`) (* 0.1 (select `bool` (> (`self.PoisonT`) 0.0) :`false` 0.0 :`true` 1.0))))
    (set `self.PoisonT` (- (`self.PoisonT`) 0.1))
    (set `self.SlowT` (- (`self.SlowT`) 0.1))
    (if (<= (`self.HP`) 0.0)
      _
      (elif (> (`self.FearT`) 0.0)
        (set `self.FearT` (- (`self.FearT`) 0.1))
        (if (> _returnvalue_2 1.0)
          (`self.K2_SetActorLocation` self (`KismetMathLibrary.MakeVector` (+ (.x _returnvalue) (* _returnvalue_3 (* 0.1 (/ (- (.x _returnvalue) (`self.FearSrcX`)) _returnvalue_2)))) (+ (.y _returnvalue) (* _returnvalue_3 (* 0.1 (/ (- (.y _returnvalue) (`self.FearSrcY`)) _returnvalue_2)))) (.z _returnvalue)) false true))
        (else
          (`/Engine/EditorBlueprintResources/StandardMacros.IsValid` (`self.TargetActor`)
            (:`Is Valid`
              (if (> (`KismetArrayLibrary.Array_Length` (`self.Path`)) (`self.PathIdx`))
                (`self.FollowPath` _returnvalue_3)
                (else
                  (`self.EngageTarget` (`self.TargetActor`) _returnvalue_3))))
            (:`Is Not Valid`
              (`self.FollowPath` _returnvalue_3))))))))

(fn `UserConstructionScript`)