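; Player controller for a tower-defense game with RTS-style unit command through a mouse cursor and a view locked to the first camera in the level.
; Left click selects units under the cursor, with Shift adding to the selection.
; Right click orders the selection to target a tower, gate, bone wall or skeleton, or otherwise move to the hit point.
; Number keys and Q forward unit spawn and cast requests to BP_TDGameDirector.
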(event `Key|LeftMouseButton`
  (params (Key :type "Key Structure"))
  (:`Pressed`
    (`self.OnLeftClick`)))

(event `self.ReceiveBeginPlay`
  (`KismetSystemLibrary.PrintString` "TDCTL alive")
  (set `self.bShowMouseCursor` true)
  (set `self.bEnableClickEvents` true)
  (set `self.bEnableMouseOverEvents` true)
  (`WidgetBlueprintLibrary.SetInputMode_GameAndUIEx` self null)
  (bind _outactors (`GameplayStatics.GetAllActorsOfClass` "/Script/Engine.CameraActor"))
  (`KismetSystemLibrary.PrintString` (`KismetStringLibrary.Concat_StrStr` "cams=" (`KismetStringLibrary.Conv_IntToString` (`KismetArrayLibrary.Array_Length` _outactors))))
  (if (> (`KismetArrayLibrary.Array_Length` _outactors) 0)
    (bind _output (`|GetArrayItem` _outactors))
    (`self.SetViewTargetWithBlend` self _output 0.5 "VTBlend_Linear" 0.0 false)
    (`KismetSystemLibrary.Delay` 0.2)
    (`self.SetViewTargetWithBlend` self _output 0.5 "VTBlend_Linear" 0.0 false)
    (`KismetSystemLibrary.PrintString` "view target set")))

(event `OnTestQ`
  (`KismetSystemLibrary.PrintString` "hi"))

(event `OnLeftClick`
  (bind _asbp_unit (cast `/Game/Blueprints/BP_Unit` (`.HitActor` (`GameplayStatics.BreakHitResult` (`self.GetHitResultUnderCursorByChannel` self "TraceTypeQuery1" false))))
    (:`then`
      (if (`self.IsInputKeyDown` self "LeftShift")
        (`KismetArrayLibrary.Array_AddUnique` (`self.SelectedUnits`) _asbp_unit)
        (else
          (`KismetArrayLibrary.Array_Clear` (`self.SelectedUnits`))
          (`KismetArrayLibrary.Array_AddUnique` (`self.SelectedUnits`) _asbp_unit))))
    (:`CastFailed`
      (`KismetArrayLibrary.Array_Clear` (`self.SelectedUnits`)))))

(event `OnRightClick`
  (bind (_hitresult _returnvalue) (`self.GetHitResultUnderCursorByChannel` self "TraceTypeQuery1" false))
  (bind (_bblockinghit _binitialoverlap _time _distance _location _impactpoint _normal _impactnormal _physmat _hitactor) (`GameplayStatics.BreakHitResult` _hitresult))
  (if (> (`KismetArrayLibrary.Array_Length` (`self.SelectedUnits`)) 0)
    (if _returnvalue
      (bind _asbp_tower (cast `/Game/Blueprints/BP_Tower` _hitactor)
        (:`then`
          (for _array_element (`self.SelectedUnits`)
            (bind _asbp_unit (cast `/Game/Blueprints/BP_Unit` _array_element))
            (`/Game/Blueprints/BP_Unit.SetTargetCommand` _asbp_unit _asbp_tower)))
        (:`CastFailed`
          (bind _asbp_gate (cast `/Game/Blueprints/BP_Gate` _hitactor)
            (:`then`
              (for _array_element_2 (`self.SelectedUnits`)
                (bind _asbp_unit_2 (cast `/Game/Blueprints/BP_Unit` _array_element_2))
                (`/Game/Blueprints/BP_Unit.SetTargetCommand` _asbp_unit_2 _asbp_gate)))
            (:`CastFailed`
              (bind _asbp_bone_wall (cast `/Game/Blueprints/BP_BoneWall` _hitactor)
                (:`then`
                  (for _array_element_3 (`self.SelectedUnits`)
                    (bind _asbp_unit_3 (cast `/Game/Blueprints/BP_Unit` _array_element_3))
                    (`/Game/Blueprints/BP_Unit.SetTargetCommand` _asbp_unit_3 _asbp_bone_wall)))
                (:`CastFailed`
                  (bind _asbp_skeleton (cast `/Game/Blueprints/BP_Skeleton` _hitactor)
                    (:`then`
                      (for _array_element_4 (`self.SelectedUnits`)
                        (bind _asbp_unit_4 (cast `/Game/Blueprints/BP_Unit` _array_element_4))
                        (`/Game/Blueprints/BP_Unit.SetTargetCommand` _asbp_unit_4 _asbp_skeleton)))
                    (:`CastFailed`
                      (for _array_element_5 (`self.SelectedUnits`)
                        (bind _asbp_unit_5 (cast `/Game/Blueprints/BP_Unit` _array_element_5))
                        (`/Game/Blueprints/BP_Unit.SetMoveCommand` _asbp_unit_5 _location)))))))))))))

(event `OnNum1`
  (bind _outactors (`GameplayStatics.GetAllActorsOfClass` "/Game/Blueprints/BP_TDGameDirector.BP_TDGameDirector_C"))
  (if (> (`KismetArrayLibrary.Array_Length` _outactors) 0)
    (bind _asbp_tdgame_director (cast `/Game/Blueprints/BP_TDGameDirector` (`|GetArrayItem` _outactors))
      (:`then`
        (`/Game/Blueprints/BP_TDGameDirector.SpawnUnit` _asbp_tdgame_director "ghoul"))
      (:`CastFailed`
        (`KismetSystemLibrary.PrintString` "Director cast failed")))))

(event `Key|RightMouseButton`
  (params (Key :type "Key Structure"))
  (:`Pressed`
    (`self.OnRightClick`)))

(event `Key|One`
  (params (Key :type "Key Structure"))
  (:`Pressed`
    (`self.OnNum1`)))

(event `OnNum2`
  (bind _outactors (`GameplayStatics.GetAllActorsOfClass` "/Game/Blueprints/BP_TDGameDirector.BP_TDGameDirector_C"))
  (if (> (`KismetArrayLibrary.Array_Length` _outactors) 0)
    (bind _asbp_tdgame_director (cast `/Game/Blueprints/BP_TDGameDirector` (`|GetArrayItem` _outactors))
      (:`then`
        (`/Game/Blueprints/BP_TDGameDirector.SpawnUnit` _asbp_tdgame_director "archer"))
      (:`CastFailed`
        (`KismetSystemLibrary.PrintString` "Director cast failed")))))

(event `Key|Two`
  (params (Key :type "Key Structure"))
  (:`Pressed`
    (`self.OnNum2`)))

(event `Key|Three`
  (params (Key :type "Key Structure"))
  (:`Pressed`
    (`self.OnNum3`)))

(event `OnNum3`
  (bind _outactors (`GameplayStatics.GetAllActorsOfClass` "/Game/Blueprints/BP_TDGameDirector.BP_TDGameDirector_C"))
  (if (> (`KismetArrayLibrary.Array_Length` _outactors) 0)
    (bind _asbp_tdgame_director (cast `/Game/Blueprints/BP_TDGameDirector` (`|GetArrayItem` _outactors))
      (:`then`
        (`/Game/Blueprints/BP_TDGameDirector.SpawnUnit` _asbp_tdgame_director "troll"))
      (:`CastFailed`
        (`KismetSystemLibrary.PrintString` "Director cast failed")))))

(event `Key|Four`
  (params (Key :type "Key Structure"))
  (:`Pressed`
    (`self.OnNum4`)))

(event `Key|Q`
  (params (Key :type "Key Structure"))
  (:`Pressed`
    (`self.OnKeyQ`)))

(event `OnNum4`
  (bind _outactors (`GameplayStatics.GetAllActorsOfClass` "/Game/Blueprints/BP_TDGameDirector.BP_TDGameDirector_C"))
  (if (> (`KismetArrayLibrary.Array_Length` _outactors) 0)
    (bind _asbp_tdgame_director (cast `/Game/Blueprints/BP_TDGameDirector` (`|GetArrayItem` _outactors))
      (:`then`
        (`/Game/Blueprints/BP_TDGameDirector.SpawnUnit` _asbp_tdgame_director "apostle"))
      (:`CastFailed`
        (`KismetSystemLibrary.PrintString` "Director cast failed")))))

(event `OnKeyQ`
  (bind _outactors (`GameplayStatics.GetAllActorsOfClass` "/Game/Blueprints/BP_TDGameDirector.BP_TDGameDirector_C"))
  (if (> (`KismetArrayLibrary.Array_Length` _outactors) 0)
    (bind _asbp_tdgame_director (cast `/Game/Blueprints/BP_TDGameDirector` (`|GetArrayItem` _outactors))
      (:`then`
        (`/Game/Blueprints/BP_TDGameDirector.CastQ` _asbp_tdgame_director))
      (:`CastFailed`
        (`KismetSystemLibrary.PrintString` "Director cast failed")))))

(fn `UserConstructionScript`)