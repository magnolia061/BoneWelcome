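; BP_Gate is a destructible gate with hit points, reporting its fall to BP_TDGameDirector.
; TakeTDamage subtracts damage from HP and, at zero or below, looks up the first director actor, calls NotifyGateDown on it, then destroys the gate.
; The gate is destroyed even if no director is found.
; TakeDmg is an empty stub, the event graph is inactive, and an unreachable older copy of the damage logic remains.
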(fn `TakeDmg`
  (params (Amount :type "Float (double-precision)")))

(fn `TakeTDamage`
  (params (N :type "Float (double-precision)"))
  (set `self.HP` (- (`self.HP`) N))
  (if (<= (`self.HP`) 0.0)
    (bind _outactors (`GameplayStatics.GetAllActorsOfClass` "/Game/Blueprints/BP_TDGameDirector.BP_TDGameDirector_C"))
    (if (> (`KismetArrayLibrary.Array_Length` _outactors) 0)
      (bind _asbp_tdgame_director (cast `/Game/Blueprints/BP_TDGameDirector` (`|GetArrayItem` _outactors))
        (:`then`
          (`/Game/Blueprints/BP_TDGameDirector.NotifyGateDown` _asbp_tdgame_director)
          (`self.K2_DestroyActor` self))
        (:`CastFailed`
          (`self.K2_DestroyActor` self)))
      (else
        (`self.K2_DestroyActor` self)))))

(fn `UserConstructionScript`)