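; Tower-defense tower that InitTower configures as arrow, poison, wail (fear) or a default skeleton-spawning tomb.
; Each type gets its own stats, cube look and looping timer that damages the nearest BP_Unit, affects units in radius, or maintains capped skeletons.
; A retry timer links it to the game director and flags high ground, widening wail radius.
; TakeTDamage handles death: stopping attacks, flattening the tower and notifying the director.
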(event `self.ReceiveBeginPlay`
  (`KismetSystemLibrary.PrintString` "tower spawned"))

(fn `ApplyToAllInRadius`
  (params (R :type "Float (double-precision)") (Mode :type Integer))
  (bind _returnvalue (`self.K2_GetActorLocation`))
  (bind _outactors (`GameplayStatics.GetAllActorsOfClass` "/Game/Blueprints/BP_Unit.BP_Unit_C"))
  (for _index (range (+ (- (`KismetArrayLibrary.Array_Length` _outactors) 1) 1))
    (bind _output (`|GetArrayItem` _outactors _index))
    (if (<= (`KismetMathLibrary.Vector_Distance2D` _returnvalue (`self.K2_GetActorLocation` _output)) R)
      (bind _asbp_unit (cast `/Game/Blueprints/BP_Unit` _output))
      (if (== Mode 0)
        (`/Game/Blueprints/BP_Unit.ApplyPoison` _asbp_unit 10.0 1.5)
        (else
          (`/Game/Blueprints/BP_Unit.ApplyFear` _asbp_unit 2.0 (.x _returnvalue) (.y _returnvalue)))))))

(fn `ArrowFire`
  (if (not (`self.bDead`))
    (bind _outactor (`self.FindNearestUnit` (`self.Range`)))
    (`/Engine/EditorBlueprintResources/StandardMacros.IsValid` _outactor
      (:`Is Valid`
        (bind _asbp_unit (cast `/Game/Blueprints/BP_Unit` _outactor))
        (`/Game/Blueprints/BP_Unit.TakeTDamage` _asbp_unit 25.0)))))

(fn `ChildDied`
  (params (S :type "Actor Object Reference"))
  (`KismetArrayLibrary.Array_RemoveItem` (`self.SkeletonsOwned`) S))

(fn `FindNearestUnit`
  (params (MaxDist :type "Float (double-precision)"))
  (returns (OutActor :type "Actor Object Reference"))
  (bind _outactors (`GameplayStatics.GetAllActorsOfClass` "/Game/Blueprints/BP_Unit.BP_Unit_C"))
  (set `self.TBestIdx` -1)
  (set `self.TBestDist` MaxDist)
  (for _index (range (+ (- (`KismetArrayLibrary.Array_Length` _outactors) 1) 1))
    (bind _returnvalue (`KismetMathLibrary.Vector_Distance2D` (`self.K2_GetActorLocation`) (`self.K2_GetActorLocation` (`|GetArrayItem` _outactors _index))))
    (if (< _returnvalue (`self.TBestDist`))
      (set `self.TBestDist` _returnvalue)
      (set `self.TBestIdx` _index)))
  (if (>= (`self.TBestIdx`) 0)
    (return (`|GetArrayItem` _outactors (`self.TBestIdx`)))
    (else
      (return null))))

(fn `InitTower`
  (params (TowerType :type Name))
  (set `self.TowerType` TowerType)
  (if (== (`self.TowerType`) "arrow")
    (set `self.MaxHP` 300.0)
    (set `self.Range` 500.0)
    (`KismetSystemLibrary.K2_SetTimer` self "ArrowFire" 1.0 true)
    (elif (== (`self.TowerType`) "poison")
      (set `self.MaxHP` 450.0)
      (set `self.Range` 300.0)
      (`KismetSystemLibrary.K2_SetTimer` self "PoisonTick" 1.0 true)
      (elif (== (`self.TowerType`) "wail")
        (set `self.MaxHP` 350.0)
        (set `self.Range` 600.0)
        (`KismetSystemLibrary.K2_SetTimer` self "WailPulse" 4.0 true)
        (else
          (set `self.MaxHP` 600.0)
          (set `self.Range` 400.0)
          (`KismetSystemLibrary.K2_SetTimer` self "RevivePulse" 6.0 true)))))
  (set `self.HP` (`self.MaxHP`))
  (`self.SetupVisual` self)
  (`KismetSystemLibrary.K2_SetTimer` self "TryLink" 0.5 true))

(fn `PoisonTick`
  (if (not (`self.bDead`))
    (`self.ApplyToAllInRadius` (`self.Range`))))

(fn `RevivePulse`
  (bind _returnvalue (`self.K2_GetActorLocation`))
  (if (`self.bDead`)
    _
    (elif (< (`KismetArrayLibrary.Array_Length` (`self.SkeletonsOwned`)) 3)
      (bind _returnvalue_2 (`|SpawnActorFromClass` "/Game/Blueprints/BP_Skeleton.BP_Skeleton_C" (`KismetMathLibrary.MakeTransform` (`KismetMathLibrary.MakeVector` (+ (.x _returnvalue) 120.0) (.y _returnvalue) 60.0)) "AlwaysSpawn" "MultiplyWithRoot" null null))
      (`KismetArrayLibrary.Array_Add` (`self.SkeletonsOwned`) _returnvalue_2)
      (bind _asbp_skeleton (cast `/Game/Blueprints/BP_Skeleton` _returnvalue_2))
      (`/Game/Blueprints/BP_Skeleton.Init` _asbp_skeleton _returnvalue)
      (set `/Game/Blueprints/BP_Skeleton.HomeTower` self _asbp_skeleton))))

(fn `SetupVisual`
  (bind _asstatic_mesh_component (cast `StaticMeshComponent` (`self.GetComponentByClass` self "/Script/Engine.StaticMeshComponent")))
  (`StaticMeshComponent.SetStaticMesh` _asstatic_mesh_component "/Engine/BasicShapes/Cube.Cube")
  (if (== (`self.TowerType`) "arrow")
    (`PrimitiveComponent.SetMaterial` _asstatic_mesh_component 0 "/Game/Materials/M_BoneTower.M_BoneTower")
    (`self.SetActorScale3D` self (`KismetMathLibrary.MakeVector` 1.2 1.2 2.6))
    (elif (== (`self.TowerType`) "poison")
      (`PrimitiveComponent.SetMaterial` _asstatic_mesh_component 0 "/Game/Materials/M_PoisonGlow.M_PoisonGlow")
      (`self.SetActorScale3D` self (`KismetMathLibrary.MakeVector` 1.3 1.3 2.2))
      (elif (== (`self.TowerType`) "wail")
        (`PrimitiveComponent.SetMaterial` _asstatic_mesh_component 0 "/Game/Materials/M_SoulGlow.M_SoulGlow")
        (`self.SetActorScale3D` self (`KismetMathLibrary.MakeVector` 1.0 1.0 3.2))
        (else
          (`PrimitiveComponent.SetMaterial` _asstatic_mesh_component 0 "/Game/Materials/M_Tomb.M_Tomb")
          (`self.SetActorScale3D` self (`KismetMathLibrary.MakeVector` 1.6 1.6 2.0)))))))

(fn `TakeDmg`
  (params (Amount :type "Float (double-precision)")))

(fn `TakeTDamage`
  (params (N :type "Float (double-precision)"))
  (bind _returnvalue (`self.GetActorScale3D`))
  (if (not (`self.bDead`))
    (set `self.HP` (- (`self.HP`) N))
    (if (<= (`self.HP`) 0.0)
      (set `self.bDead` true)
      (`KismetSystemLibrary.K2_ClearTimer` self "ArrowFire")
      (`KismetSystemLibrary.K2_ClearTimer` self "PoisonTick")
      (`KismetSystemLibrary.K2_ClearTimer` self "WailPulse")
      (`KismetSystemLibrary.K2_ClearTimer` self "RevivePulse")
      (`self.SetActorScale3D` self (`KismetMathLibrary.MakeVector` (.x _returnvalue) (.y _returnvalue) (* (.z _returnvalue) 0.25)))
      (bind _asbp_tdgame_director (cast `/Game/Blueprints/BP_TDGameDirector` (`self.Director`)))
      (`/Game/Blueprints/BP_TDGameDirector.NotifyTowerDown` _asbp_tdgame_director self))))

(fn `TryLink`
  (bind _returnvalue (`self.K2_GetActorLocation`))
  (`/Engine/EditorBlueprintResources/StandardMacros.IsValid` (`self.Director`)
    (:`Is Valid`
      (bind _asbp_tdgame_director (cast `/Game/Blueprints/BP_TDGameDirector` (`self.Director`)))
      (`/Game/Blueprints/BP_TDGameDirector.RegisterTower` _asbp_tdgame_director self)
      (bind _char (`/Game/Blueprints/BP_TDGameDirector.TileChar` _asbp_tdgame_director (`KismetMathLibrary.FFloor` (/ (.x _returnvalue) 100.0)) (`KismetMathLibrary.FFloor` (/ (.y _returnvalue) 100.0))))
      (if (`KismetStringLibrary.EqualEqual_StrStr` _char "^")
        (set `self.bOnHighGround` true))
      (`KismetSystemLibrary.K2_ClearTimer` self "TryLink"))
    (:`Is Not Valid`
      (bind _asbp_tdplayer_controller (cast `/Game/Blueprints/BP_TDPlayerController` (`GameplayStatics.GetPlayerController` 0)))
      (set `self.Director` (`/Game/Blueprints/BP_TDPlayerController.Director` _asbp_tdplayer_controller)))))

(fn `UserConstructionScript`)

(fn `WailPulse`
  (if (not (`self.bDead`))
    (`self.ApplyToAllInRadius` (select `bool` (`self.bOnHighGround`) :`false` 600.0 :`true` 800.0) 1)))